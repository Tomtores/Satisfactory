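; Interactable foliage ghost actor that a player can use to delete it from the world.
; It shows a hologram outline on its static mesh from BeginPlay and switches to the dismantle color while looked at.
; On use it calls RemoveFromWorld, defined outside these graphs, and logs success or failure plus the returned log.
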(event `FGUseableInterface.OnUse`
  (params (byCharacter :type "FGCharacterPlayer Object Reference") (state :type "UseState Structure (by ref)"))
  (bind (_log _returnvalue) (`self.RemoveFromWorld` (`self.Debug`)))
  (if _returnvalue
    (`BlueprintLoggingLibrary.LogDisplay` "Foliage Ghost Actor removed.")
    (else
      (`BlueprintLoggingLibrary.LogError` "Foliage Ghost Actor not removed.")))
  (`BlueprintLoggingLibrary.LogDisplay` _log))

(event `FGUseableInterface.StartIsLookedAt`
  (params (byCharacter :type "FGCharacterPlayer Object Reference") (state :type "UseState Structure (by ref)"))
  (`FGBlueprintFunctionLibrary.ShowOutline` (`self.StaticMeshComponent`) "OC_DISMANTLE"))

(event `FGUseableInterface.StopIsLookedAt`
  (params (byCharacter :type "FGCharacterPlayer Object Reference") (state :type "UseState Structure (by ref)"))
  (`FGBlueprintFunctionLibrary.ShowOutline` (`self.StaticMeshComponent`) "OC_HOLOGRAM" :!label _label))

(event `self.ReceiveBeginPlay`
  (goto _label))

(fn `GetLookAtDecription`
  (params (byCharacter :type "FGCharacterPlayer Object Reference") (state :type "UseState Structure (by ref)"))
  (returns (ReturnValue :type Text))
  (return "Foliage ghost, interact to delete"))

(fn `IsUseable`
  (returns (ReturnValue :type Boolean))
  (return true))

(fn `ShouldBlockInteraction`
  (params (byCharacter :type "FGCharacterPlayer Object Reference") (hitResult :type "HitResult Structure (by ref)"))
  (returns (ReturnValue :type Boolean))
  (return false))

(fn `UpdateUseState`
  (params (byCharacter :type "FGCharacterPlayer Object Reference") (atLocation :type "Vector Structure (by ref)") (componentHit :type "PrimitiveComponent Object Reference") (out_useState :type "UseState Structure (by ref)"))
  (return))

(fn `UserConstructionScript`)